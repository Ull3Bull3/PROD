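; Monster spawn point actor that tracks a current spawn location and advances it through three fixed stages.
; BeginPlay takes the Cube's world position as the initial location and converts the Location1 and LocationFinal offsets into world positions relative to it.
; Each UpdateSpawnLocation call compares the current location with zero tolerance to pick the next stage, printing its name and stopping at the final one.
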(event `UpdateSpawnLocation`
  (if (== (`self.SpawnLocation`) (`self.Location_0`))
    (set `self.SpawnLocation` (`self.Location_1`))
    (`KismetSystemLibrary.PrintString` "Location 1")
    (elif (== (`self.SpawnLocation`) (`self.Location_1`))
      (set `self.SpawnLocation` (`self.Location_Final`))
      (`KismetSystemLibrary.PrintString` "Location Final"))))

(event `self.ReceiveBeginPlay`
  (bind _returnvalue (`SceneComponent.K2_GetComponentLocation` (`self.Cube`)))
  (`|ExecutionSequence`
    (:`then_0`
      (set `self.Location_0` _returnvalue)
      (set `self.SpawnLocation` (`self.Location_0`)))
    (:`then_1`
      (set `self.Location_1` (+ _returnvalue (`self.Location_1`))))
    (:`then_2`
      (set `self.Location_Final` (+ _returnvalue (`self.Location_Final`))))))

(event `self.ReceiveActorBeginOverlap`
  (params (OtherActor :type "Actor Object Reference")))

(fn `UserConstructionScript`)