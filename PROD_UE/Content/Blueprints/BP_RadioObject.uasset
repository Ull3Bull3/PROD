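; BP_RadioObject is an interactable radio that emits a beeping sound until the Interact event stops it.
; A DoOnce on Tick, rather than BeginPlay, spawns the sound attached to the box collision and keeps the audio component reference for stopping.
; The same box shows InteractText while the first-person character overlaps it and hides it on exit.
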(event `self.ReceiveTick`
  (params (DeltaSeconds :type "Float (single-precision)"))
  (`/Engine/EditorBlueprintResources/StandardMacros.DoOnce` false
    (:`Completed`
      (bind _returnvalue (`GameplayStatics.SpawnSoundAttached` "/Game/Sounds/radio_beep.radio_beep" (`self.BoxCollision`) "None" (0.0 0.0 0.0) (struct) "KeepRelativeOffset" false 1.0 1.0 0.0 "/Game/Sounds/Attenuation/ATT_Radio_Beep.ATT_Radio_Beep" null)))))

(event `/Game/Blueprints/BP_KeyInterface.Interact`
  (`KismetSystemLibrary.PrintString` "interact radio")
  (`AudioComponent.Stop` (stale `self.ReceiveTick` _returnvalue)))

(event `self.BoxCollision.OnComponentBeginOverlap`
  (params (OverlappedComponent :type "PrimitiveComponent Object Reference") (OtherActor :type "Actor Object Reference") (OtherComp :type "PrimitiveComponent Object Reference") (OtherBodyIndex :type Integer) (bFromSweep :type Boolean) (SweepResult :type "HitResult Structure (by ref)"))
  ;[1 1 1] Text
  (cast `/Game/FirstPerson/Blueprints/BP_FirstPersonCharacter` OtherActor)
  (`SceneComponent.SetHiddenInGame` (`self.InteractText`) false false))

(event `self.BoxCollision.OnComponentEndOverlap`
  (params (OverlappedComponent :type "PrimitiveComponent Object Reference") (OtherActor :type "Actor Object Reference") (OtherComp :type "PrimitiveComponent Object Reference") (OtherBodyIndex :type Integer))
  ;[1 1 1] Text
  (cast `/Game/FirstPerson/Blueprints/BP_FirstPersonCharacter` OtherActor)
  (`SceneComponent.SetHiddenInGame` (`self.InteractText`) true false))

(fn `UserConstructionScript`)