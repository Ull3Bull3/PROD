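; BP_Key_3DSound is an actor, named as a key's 3D sound, that sweeps from the player's left to their right.
; BeginPlay sets a start point to the left of the player pawn along its right vector.
; Tick moves the actor at constant speed toward a target on the right, recomputed each frame from the pawn's current position and facing.
; A DestroySound event destroys the actor.
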(event `self.ReceiveBeginPlay`
  (bind _returnvalue (`GameplayStatics.GetPlayerPawn` 0))
  (set `self.CurrentPosition` (+ (* (`self.GetActorRightVector` _returnvalue) -200.0) (`self.K2_GetActorLocation` _returnvalue))))

(event `self.ReceiveTick`
  (params (DeltaSeconds :type "Float (single-precision)"))
  (bind _returnvalue (`GameplayStatics.GetPlayerPawn` 0))
  (bind _output_get (set `self.CurrentPosition` (`KismetMathLibrary.VInterpTo_Constant` (`self.CurrentPosition`) (+ (* (`self.GetActorRightVector` _returnvalue) 200.0) (`self.K2_GetActorLocation` _returnvalue)) DeltaSeconds 80.0)))
  (`self.K2_SetActorLocation` _output_get))

(event `DestroySound`
  (`self.K2_DestroyActor`))

(fn `UserConstructionScript`)