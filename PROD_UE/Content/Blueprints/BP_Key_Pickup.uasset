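; BP_Key_Pickup is an interactable electrical key that launches a minigame to open its linked door.
; Overlapping its box shows interact text while the door is closed; Interact creates WBP_Key_Minigame, locks player input and stops the attached sparking loop.
; Success opens the door, optionally updates the objective and spawns a monster.
; A reset re-arms the DoOnce-gated sound and interaction and plays a throttled failure voice line.
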(event `self.ReceiveTick`
  (params (DeltaSeconds :type "Float (single-precision)"))
  ;[1 1 1] Play Sparking Sound
  (`/Engine/EditorBlueprintResources/StandardMacros.DoOnce` false :!label _label
    (:`Completed`
      (bind _returnvalue (`GameplayStatics.SpawnSoundAttached` "/Game/Sounds/Electricity_Sparks.Electricity_Sparks" (`self.BoxCollision`) "None" (0.0 0.0 0.0) (struct) "KeepRelativeOffset" false (`self.Volume Multiplier`) 1.0 0.0 "/Game/Sounds/Attenuation/ATT_Electricity_Sparks.ATT_Electricity_Sparks" null)))))

(event `/Game/Blueprints/BP_KeyInterface.Interact`
  ;[1 1 1] Interact Key
  (`/Engine/EditorBlueprintResources/StandardMacros.DoOnce` false :!label _label_2
    (:`Completed`
      (bind _returnvalue (`|CreateWidget` "/Game/Blueprints/WBP_Key_Minigame.WBP_Key_Minigame_C"))
      (bind _output_get (set `self.KeyWidget` _returnvalue))
      (set `/Game/Blueprints/WBP_Key_Minigame.Key_Pickup` self _output_get)
      (`UserWidget.AddToViewport` _output_get 0)
      (`self.DisablePlayerInput`)
      (message `/Game/Blueprints/BPI_Logging.Log Data` (`GameplayStatics.GetGameMode`) "Started Key Minigame")
      (`AudioComponent.Stop` (stale `self.ReceiveTick` _returnvalue)))))

(event `ShouldResetKey`
  ;[1 1 1] Reset Key
  (if (not (`/Game/Blueprints/BP_Door.DoorOpen` (`self.Door`)))
    ;[1 1 1] Interact Key
    (`|ExecutionSequence`
      (:`then_0`
        (goto _label :!via `Reset`))
      (:`then_1`
        (goto _label_2 :!via `Reset`))
      (:`then_2`
        (if (not (`self.bPlayerVoiceLinePlaying`))
          (set `self.bPlayerVoiceLinePlaying` true)
          (`GameplayStatics.PlaySound2D` "/Game/Sounds/Voice/PlayerFailElectricMinigame.PlayerFailElectricMinigame" 1.0 1.0 0.0 null null)
          (`KismetSystemLibrary.Delay` (`self.VoiceLineTimer`))
          (set `self.bPlayerVoiceLinePlaying` false))))))

(event `self.BoxCollision.OnComponentBeginOverlap`
  (params (OverlappedComponent :type "PrimitiveComponent Object Reference") (OtherActor :type "Actor Object Reference") (OtherComp :type "PrimitiveComponent Object Reference") (OtherBodyIndex :type Integer) (bFromSweep :type Boolean) (SweepResult :type "HitResult Structure (by ref)"))
  ;[1 1 1] Text
  (if (not (`/Game/Blueprints/BP_Door.DoorOpen` (`self.Door`)))
    (cast `/Game/FirstPerson/Blueprints/BP_FirstPersonCharacter` OtherActor)
    (`SceneComponent.SetHiddenInGame` (`self.InteractText`) false false)
    (`GameplayStatics.PlaySound2D` "/Game/Sounds/Interactable.Interactable" 1.0 1.0 0.0 null null)))

(event `ShouldOpenDoor`
  (bind _changeplayerobjective (`self.ChangePlayerObjective`))
  ;[1 1 1] Open Door
  (bind _asbp_door (cast `/Game/Blueprints/BP_Door` (`self.Door`))
    (:`then`
      (`/Game/Blueprints/BP_Door.OpenDoor` _asbp_door)
      (`GameplayStatics.PlaySound2D` "/Game/Sounds/Electricity_Success.Electricity_Success" 1.0 1.0 0.0 null null)
      (`|ExecutionSequence`
        (:`then_0`
          (`/Engine/EditorBlueprintResources/StandardMacros.IsValid` (`/Game/Blueprints/ActorComponents/ChangePlayerObjective.NewObjective` _changeplayerobjective)
            (:`Is Valid`
              (`/Game/Blueprints/ActorComponents/ChangePlayerObjective.Update Player Objective` _changeplayerobjective))))
        (:`then_1`
          (if (`self.ShouldSpawnMonster`)
            (bind _returnvalue (`GameplayStatics.GetActorOfClass` "/Game/Blueprints/Monster/BP_MonsterSpawner.BP_MonsterSpawner_C"))
            (`/Game/Blueprints/Monster/BP_MonsterSpawner.Spawn Monster` _returnvalue)
            (`GameplayStatics.PlaySound2D` (`self.VoiceLine_ForMonster_Trigger`) 1.0 1.0 0.0 null null)))))
    (:`CastFailed`
      (`KismetSystemLibrary.PrintString` "Door Cast Failed, No door placed in key"))))

(event `self.BoxCollision.OnComponentEndOverlap`
  (params (OverlappedComponent :type "PrimitiveComponent Object Reference") (OtherActor :type "Actor Object Reference") (OtherComp :type "PrimitiveComponent Object Reference") (OtherBodyIndex :type Integer))
  ;[1 1 1] Text
  (cast `/Game/FirstPerson/Blueprints/BP_FirstPersonCharacter` OtherActor)
  (`SceneComponent.SetHiddenInGame` (`self.InteractText`) true false))

(event `DisablePlayerInput`
  (bind _returnvalue (`GameplayStatics.GetPlayerController` 0))
  ;[1 1 1] Disable Move and Rotation Input during minigame
  (`Controller.SetIgnoreMoveInput` _returnvalue true)
  (`Controller.SetIgnoreLookInput` _returnvalue true))

(fn `UserConstructionScript`)