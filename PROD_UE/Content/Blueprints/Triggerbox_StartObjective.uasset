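; Trigger box that sets the player's starting objective and configures the monster spawner when the player pawn overlaps it.
; On Tick it checks the overlap, writes PlayerObjective to BP_FirstPersonCharacter, then passes its spawn and end points to BP_MonsterSpawner.
; The non-overlap branch also destroys the actor, so it only takes effect if the player is inside on its first tick.
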(event `self.ReceiveTick`
  (params (DeltaSeconds :type "Float (single-precision)"))
  (bind _returnvalue (`GameplayStatics.GetPlayerPawn` 0))
  ;[1 1 1] Sets first player objective, then destroys itself
  (if (`self.IsOverlappingActor` _returnvalue)
    (`|ExecutionSequence`
      (:`then_0`
        (bind _asbp_first_person_character (cast `/Game/FirstPerson/Blueprints/BP_FirstPersonCharacter` _returnvalue)
          (:`then`
            (set `/Game/FirstPerson/Blueprints/BP_FirstPersonCharacter.CurrentObjective` (`self.PlayerObjective`) _asbp_first_person_character))
          (:`CastFailed`
            _))
        (`self.K2_DestroyActor` :!label _label))
      (:`then_1`
        (bind _returnvalue_2 (`GameplayStatics.GetActorOfClass` "/Game/Blueprints/BP_MonsterSpawner.BP_MonsterSpawner_C"))
        (`|ExecutionSequence`
          (:`then_0`
            (set `/Game/Blueprints/BP_MonsterSpawner.CurrentSpawnPoint` (`self.MonsterSpawnPoint`) _returnvalue_2))
          (:`then_1`
            (set `/Game/Blueprints/BP_MonsterSpawner.CurrentEndPoint` (`self.MonsterEndPoint`) _returnvalue_2)))))
    (else
      (goto _label))))

(fn `UserConstructionScript`)