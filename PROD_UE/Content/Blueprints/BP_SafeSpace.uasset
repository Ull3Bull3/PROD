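; Safe zone actor that flags the first-person player as safe while they overlap it.
; BeginPlay attaches an attenuated fireplace sound to its cube.
; Player entry sets IsInSafeSpace on BP_FirstPersonCharacter through SetPlayerSafe, attaches a choir sound and plays a 2D enter cue.
; Exit clears the flag and fades out the choir over a second.
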(event `self.ReceiveBeginPlay`
  (`GameplayStatics.SpawnSoundAttached` "/Game/Sounds/Fireplace_SafeSpace.Fireplace_SafeSpace" (`self.Cube`) "None" (0.0 0.0 0.0) (struct) "KeepRelativeOffset" false 1.0 1.0 0.0 "/Game/Sounds/Attenuation/ATT_SafeSpace.ATT_SafeSpace" null false))

(event `self.ReceiveActorBeginOverlap`
  (params (OtherActor :type "Actor Object Reference"))
  (bind _returnvalue (`GameplayStatics.GetPlayerPawn` 0))
  (if (== OtherActor _returnvalue)
    (bind _asbp_first_person_character (cast `/Game/FirstPerson/Blueprints/BP_FirstPersonCharacter` _returnvalue))
    (`self.SetPlayerSafe` true _asbp_first_person_character)
    (bind _returnvalue_2 (`GameplayStatics.SpawnSoundAttached` "/Game/Sounds/Choir.Choir" (`self.Cube`) "None" (0.0 0.0 0.0) (struct) "KeepRelativeOffset" false 1.0 1.0 0.0 "/Game/Sounds/Attenuation/ATT_SafeSpace.ATT_SafeSpace" null))
    (`GameplayStatics.PlaySound2D` "/Game/Sounds/SafeZoneEnter.SafeZoneEnter" 1.0 1.0 0.0 null null)))

(event `self.ReceiveActorEndOverlap`
  (params (OtherActor :type "Actor Object Reference"))
  (bind _returnvalue (`GameplayStatics.GetPlayerPawn` 0))
  (if (== OtherActor _returnvalue)
    (bind _asbp_first_person_character (cast `/Game/FirstPerson/Blueprints/BP_FirstPersonCharacter` _returnvalue))
    (`self.SetPlayerSafe` false _asbp_first_person_character)
    (`/Engine/EditorBlueprintResources/StandardMacros.IsValid` (stale `self.ReceiveActorBeginOverlap` _returnvalue_2)
      (:`Is Valid`
        (`AudioComponent.FadeOut` (stale `self.ReceiveActorBeginOverlap` _returnvalue_2) 1.0 0.0 "Linear")))))

(fn `SetPlayerSafe`
  (params (bIsPlayerSafe :type Boolean) (Player :type "/Game/FirstPerson/Blueprints/BP_FirstPersonCharacter Object Reference"))
  (set `/Game/FirstPerson/Blueprints/BP_FirstPersonCharacter.IsInSafeSpace` bIsPlayerSafe Player))

(fn `UserConstructionScript`)