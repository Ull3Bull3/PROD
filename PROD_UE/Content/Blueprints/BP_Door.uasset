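; BP_Door is a key-gated door actor that opens once enough keys are counted.
; Each OpenDoor event increments CurrentKeys; on reaching KeyAmountToOpen, it flags DoorOpen and snaps DoorMesh to a fixed relative open pose, without interpolation.
; A DoOnce limits the attenuated opening sound to a single play.
; Hit and end-overlap events toggle DoorSlideBool, which nothing in these graphs reads.
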(event `self.ReceiveHit`
  (params (MyComp :type "PrimitiveComponent Object Reference") (Other :type "Actor Object Reference") (OtherComp :type "PrimitiveComponent Object Reference") (bSelfMoved :type Boolean) (HitLocation :type "Vector Structure") (HitNormal :type "Vector Structure") (NormalImpulse :type "Vector Structure") (Hit :type "HitResult Structure (by ref)"))
  (set `self.DoorSlideBool` true))

(event `self.ReceiveActorEndOverlap`
  (params (OtherActor :type "Actor Object Reference"))
  (set `self.DoorSlideBool` false))

(event `self.ReceiveTick`
  (params (DeltaSeconds :type "Float (single-precision)")))

(event `OpenDoor`
  ;[1 1 1] Open Door
  (set `self.CurrentKeys` (+ (`self.CurrentKeys`) 1))
  (if (>= (`self.CurrentKeys`) (`self.KeyAmountToOpen`))
    (set `self.DoorOpen` true)
    (`SceneComponent.K2_SetRelativeLocationAndRotation` (`self.DoorMesh`) (60.0 -60.0 0.0) (`KismetMathLibrary.MakeRotator` 0.0 0.0 -90.0) false false)
    (`/Engine/EditorBlueprintResources/StandardMacros.DoOnce` false
      (:`Completed`
        (`GameplayStatics.SpawnSoundAttached` "/Game/Sounds/Door_opening.Door_opening" (`self.DoorMesh`) "None" (0.0 0.0 0.0) (struct) "KeepRelativeOffset" false 1.0 1.0 0.0 "/Game/Sounds/Attenuation/ATT_Door.ATT_Door" null)))))

(fn `UserConstructionScript`)