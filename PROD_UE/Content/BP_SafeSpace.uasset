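; BP_SafeSpace is a zone actor that marks the player as safe while they are inside it.
; On begin and end overlap it checks that the other actor is player pawn 0 and casts it to BP_FirstPersonCharacter.
; A SetPlayerSafe function then writes true or false to the character's IsInSafeSpace flag.
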(event `self.ReceiveActorBeginOverlap`
  (params (OtherActor :type "Actor Object Reference"))
  (bind _returnvalue (`GameplayStatics.GetPlayerPawn` 0))
  (if (== OtherActor _returnvalue)
    (bind _asbp_first_person_character (cast `/Game/FirstPerson/Blueprints/BP_FirstPersonCharacter` _returnvalue))
    (`self.SetPlayerSafe` true _asbp_first_person_character)))

(event `self.ReceiveActorEndOverlap`
  (params (OtherActor :type "Actor Object Reference"))
  (bind _returnvalue (`GameplayStatics.GetPlayerPawn` 0))
  (if (== OtherActor _returnvalue)
    (bind _asbp_first_person_character (cast `/Game/FirstPerson/Blueprints/BP_FirstPersonCharacter` _returnvalue))
    (`self.SetPlayerSafe` false _asbp_first_person_character)))

(fn `SetPlayerSafe`
  (params (bIsPlayerSafe :type Boolean) (Player :type "/Game/FirstPerson/Blueprints/BP_FirstPersonCharacter Object Reference"))
  (set `/Game/FirstPerson/Blueprints/BP_FirstPersonCharacter.IsInSafeSpace` bIsPlayerSafe Player))

(fn `UserConstructionScript`)