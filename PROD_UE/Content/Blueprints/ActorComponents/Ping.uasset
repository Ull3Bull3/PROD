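; Ping is an actor component that plays audio cues at its owning actor's location on demand.
; PlayPingSound fires a one-shot low-pitch ping.
; PlayAmbientSound spawns the objective ambience and prints a debug "Hello", while StopAmbientSound briefly fades out that spawned audio component if it is still valid.
; Both sounds start at the owner's position at call time and are not attached to it.
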(event `Play Ping Sound`
  ;[1 1 1] Plays a ping sound on demand on the location of the actor
  (`GameplayStatics.PlaySoundAtLocation` "/Game/Sounds/Ping_Low_Pitch.Ping_Low_Pitch" (`Actor.K2_GetActorLocation` (`self.GetOwner` self)) (struct) 1.0 1.0 0.0 "/Game/Sounds/Attenuation/ATT_Ping_Low_Pitch.ATT_Ping_Low_Pitch" null null null))

(event `Play Ambient Sound`
  (bind _returnvalue (`GameplayStatics.SpawnSoundAtLocation` "/Game/Sounds/Objective_Ambience.Objective_Ambience" (`Actor.K2_GetActorLocation` (`self.GetOwner` self)) (struct) 1.0 1.0 0.0 "/Game/Sounds/Attenuation/ATT_Ping_Low_Pitch.ATT_Ping_Low_Pitch" null))
  (`KismetSystemLibrary.PrintString` "Hello"))

(event `Stop Ambient Sound`
  (`/Engine/EditorBlueprintResources/StandardMacros.IsValid` (stale `Play Ambient Sound` _returnvalue)
    (:`Is Valid`
      (`AudioComponent.FadeOut` (stale `Play Ambient Sound` _returnvalue) 0.2 0.0 "Linear"))))