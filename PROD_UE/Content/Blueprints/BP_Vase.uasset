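; Vase actor that wobbles when the first-person player enters its trigger box and can set off a monster spawn.
; After a short delay on BeginPlay, it copies the vase message time from the game mode into FallTime.
; The trigger overlap passes the player's CharacterMovement to Wobble, whose logic is not in these graphs.
; OnLog forwards text to the game mode's logger, and SpawnMonster calls the level's BP_MonsterSpawner.
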(event `self.ReceiveBeginPlay`
  (`KismetSystemLibrary.Delay` 0.2)
  (bind _timetosavevase (message `/Game/Blueprints/BPI_JsonVariables.GetTimeForVase` (`GameplayStatics.GetGameMode`)))
  (set `self.FallTime` _timetosavevase))

(event `self.ReceiveTick`
  (params (DeltaSeconds :type "Float (single-precision)")))

(event `self.OnLog`
  (params (LogText :type String))
  (message `/Game/Blueprints/BPI_Logging.Log Data` (`GameplayStatics.GetGameMode`) LogText))

(event `self.TriggerBox.OnComponentBeginOverlap`
  (params (OverlappedComponent :type "PrimitiveComponent Object Reference") (OtherActor :type "Actor Object Reference") (OtherComp :type "PrimitiveComponent Object Reference") (OtherBodyIndex :type Integer) (bFromSweep :type Boolean) (SweepResult :type "HitResult Structure (by ref)"))
  (bind _asbp_first_person_character (cast `/Game/FirstPerson/Blueprints/BP_FirstPersonCharacter` OtherActor))
  (`self.Wobble` (`Character.CharacterMovement` _asbp_first_person_character)))

(event `self.SpawnMonster`
  (bind _returnvalue (`GameplayStatics.GetActorOfClass` "/Game/Blueprints/Monster/BP_MonsterSpawner.BP_MonsterSpawner_C"))
  (`/Game/Blueprints/Monster/BP_MonsterSpawner.Spawn Monster` _returnvalue))

(fn `UserConstructionScript`)