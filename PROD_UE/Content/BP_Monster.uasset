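; BP_Monster is a monster that attacks the player on a repeating cooldown, with outcomes only printed as debug strings.
; Tick counts the cooldown down, announces an attack, and parks the timer at a high placeholder while a delay runs.
; After the delay it restores the base cooldown and checks the first-person character's IsInSafeSpace flag to report safety or damage.
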(event `self.ReceiveTick`
  (params (DeltaSeconds :type "Float (single-precision)"))
  (bind _output_get (set `self.AttackCooldown` (- (`self.AttackCooldown`) DeltaSeconds)))
  (if (<= _output_get 0.0)
    (`KismetSystemLibrary.PrintString` "Monster Attacks")
    (set `self.AttackCooldown` 100.0)
    (bind _asbp_first_person_character (cast `/Game/FirstPerson/Blueprints/BP_FirstPersonCharacter` (`GameplayStatics.GetPlayerPawn` 0)))
    (`KismetSystemLibrary.Delay` (`self.AttackDelay`))
    (set `self.AttackCooldown` (`self.BaseAttackCooldown`))
    (if (`/Game/FirstPerson/Blueprints/BP_FirstPersonCharacter.IsInSafeSpace` _asbp_first_person_character)
      (`KismetSystemLibrary.PrintString` "Player is Safe! ")
      (else
        (`KismetSystemLibrary.PrintString` "Player Takes Damage")))))

(fn `UserConstructionScript`)