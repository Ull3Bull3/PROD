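; Monster actor that sweeps toward an end point, killing the first-person player on overlap unless they are in a safe space.
; On spawn it starts the player's breathing, waits a start delay, then plays attached sounds and takes its end point from BP_MonsterSpawner.
; Tick moves it at constant game-mode speed, yawed toward that point; reaching it or killing the player destroys it.
; Spawn, survival and death are logged through the game mode.
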(event `self.ReceiveBeginPlay`
  (bind _box (`self.Box`))
  (bind _asbp_first_person_character (cast `/Game/FirstPerson/Blueprints/BP_FirstPersonCharacter` (`GameplayStatics.GetPlayerPawn` 0)))
  (`/Game/FirstPerson/Blueprints/BP_FirstPersonCharacter.StartBreathing` _asbp_first_person_character)
  (`KismetSystemLibrary.Delay` (`self.StartTime`))
  (set `self.StartMoving` true)
  (`GameplayStatics.SpawnSoundAttached` "/Game/Sounds/Monster_Howl.Monster_Howl" _box "None" (0.0 0.0 0.0) (struct) "KeepRelativeOffset" true 1.0 1.0 0.0 "/Game/Sounds/Attenuation/ATT_Monster.ATT_Monster" null)
  (`GameplayStatics.SpawnSoundAttached` "/Game/Sounds/Monster_Scream.Monster_Scream" _box "None" (0.0 0.0 0.0) (struct) "KeepRelativeOffset" true 0.7 1.0 0.0 "/Game/Sounds/Attenuation/ATT_Monster.ATT_Monster" null)
  (`GameplayStatics.SpawnSoundAttached` "/Game/Sounds/Monster_Storm.Monster_Storm" _box "None" (0.0 0.0 0.0) (struct) "KeepRelativeOffset" true 0.5 1.0 0.0 "/Game/Sounds/Attenuation/ATT_Monster.ATT_Monster" null)
  (message `/Game/Blueprints/BPI_Logging.Log Data` (`GameplayStatics.GetGameMode`) "Monster Spawned")
  (bind _returnvalue (`GameplayStatics.GetActorOfClass` "/Game/Blueprints/Monster/BP_MonsterSpawner.BP_MonsterSpawner_C"))
  (set `self.End Point` (`/Game/Blueprints/Monster/BP_MonsterSpawner.CurrentEndPoint` _returnvalue)))

(event `self.ReceiveActorBeginOverlap`
  (params (OtherActor :type "Actor Object Reference"))
  (bind _returnvalue (`GameplayStatics.GetGameMode`))
  (`|ExecutionSequence`
    (:`then_0`
      (bind _asbp_first_person_character (cast `/Game/FirstPerson/Blueprints/BP_FirstPersonCharacter` OtherActor))
      (if (`/Game/FirstPerson/Blueprints/BP_FirstPersonCharacter.IsInSafeSpace` _asbp_first_person_character)
        (message `/Game/Blueprints/BPI_Logging.Log Data` _returnvalue "Player Survived")
        (else
          (`/Game/FirstPerson/Blueprints/BP_FirstPersonCharacter.Death Sequence` _asbp_first_person_character)
          (message `/Game/Blueprints/BPI_Logging.Log Data` _returnvalue "Player Died")
          (`self.K2_DestroyActor`))))
    (:`then_1`
      (if (== (`self.End Point`) OtherActor)
        (`GameplayStatics.PlaySoundAtLocation` "/Game/Sounds/Monster_Disappear.Monster_Disappear" (`self.K2_GetActorLocation`) (struct) 2.0 1.0 0.0 "/Game/Sounds/Attenuation/ATT_Monster.ATT_Monster" null null null)
        (`self.K2_DestroyActor`)))))

(event `self.ReceiveTick`
  (params (DeltaSeconds :type "Float (single-precision)"))
  (bind _defaultsceneroot (`self.DefaultSceneRoot`))
  (bind (_returnvalue_roll _returnvalue_pitch) (`KismetMathLibrary.BreakRotator` (`SceneComponent.K2_GetComponentRotation` _defaultsceneroot)))
  (bind (_returnvalue_roll_2 _returnvalue_pitch_2 _returnvalue_yaw) (`KismetMathLibrary.BreakRotator` (`KismetMathLibrary.FindLookAtRotation` (`SceneComponent.K2_GetComponentLocation` _defaultsceneroot) (`SceneComponent.K2_GetComponentLocation` (`/Game/Blueprints/Monster/BP_MonsterEndPoint1.DefaultSceneRoot` (`self.End Point`))))))
  (if (`self.StartMoving`)
    (`|ExecutionSequence`
      (:`then_0`
        (bind _enemyspeed (message `/Game/Blueprints/BPI_JsonVariables.GetEnemySpeed` (`GameplayStatics.GetGameMode`)))
        (`self.K2_SetActorLocation` (`KismetMathLibrary.VInterpTo_Constant` (`self.K2_GetActorLocation`) (`self.K2_GetActorLocation` (`self.End Point`)) DeltaSeconds _enemyspeed)))
      (:`then_1`
        (`/Engine/EditorBlueprintResources/StandardMacros.IsValid` _defaultsceneroot
          (:`Is Valid`
            (`SceneComponent.K2_SetWorldRotation` _defaultsceneroot (`KismetMathLibrary.MakeRotator` _returnvalue_roll _returnvalue_pitch _returnvalue_yaw) false false)))))))

(fn `UserConstructionScript`)