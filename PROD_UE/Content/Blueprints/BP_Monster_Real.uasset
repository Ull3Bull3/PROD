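; BP_Monster_Real is a lethal roaming monster that restarts the current level when it overlaps a player who is not in a safe space.
; After a StartTime delay it plays attached howl, scream and storm sounds and starts moving.
; Tick moves it at constant speed toward the CurrentEndPoint of BP_MonsterSpawner, looked up every frame.
; Overlapping BP_MonsterEndPoint1 plays a disappear sound at world origin and destroys it.
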(event `self.ReceiveActorBeginOverlap`
  (params (OtherActor :type "Actor Object Reference"))
  (`|ExecutionSequence`
    (:`then_0`
      (bind _asbp_first_person_character (cast `/Game/FirstPerson/Blueprints/BP_FirstPersonCharacter` OtherActor))
      (if (`/Game/FirstPerson/Blueprints/BP_FirstPersonCharacter.IsInSafeSpace` _asbp_first_person_character)
        (`KismetSystemLibrary.PrintString` "Player is Safe! ")
        (else
          (bind _returnvalue (`GameplayStatics.GetCurrentLevelName` true))
          (`GameplayStatics.OpenLevel` (`KismetStringLibrary.Conv_StringToName` _returnvalue)))))
    (:`then_1`
      (cast `/Game/Blueprints/BP_MonsterEndPoint1` OtherActor)
      (`GameplayStatics.PlaySoundAtLocation` "/Game/Sounds/Monster_Disappear.Monster_Disappear" (0.0 0.0 0.0) (struct) 2.0 1.0 0.0 "/Game/Sounds/Attenuation/ATT_Monster.ATT_Monster" null null null)
      (`self.K2_DestroyActor`))))

(event `self.ReceiveBeginPlay`
  (bind _box (`self.Box`))
  (`KismetSystemLibrary.PrintString` "BEgingpLay")
  (`KismetSystemLibrary.Delay` (`self.StartTime`))
  (set `self.StartMoving` true)
  (`GameplayStatics.SpawnSoundAttached` "/Game/Sounds/Monster_Howl.Monster_Howl" _box "None" (0.0 0.0 0.0) (struct) "KeepRelativeOffset" true 1.0 1.0 0.0 "/Game/Sounds/Attenuation/ATT_Monster.ATT_Monster" null)
  (`GameplayStatics.SpawnSoundAttached` "/Game/Sounds/Monster_Scream.Monster_Scream" _box "None" (0.0 0.0 0.0) (struct) "KeepRelativeOffset" true 0.7 1.0 0.0 "/Game/Sounds/Attenuation/ATT_Monster.ATT_Monster" null)
  (`GameplayStatics.SpawnSoundAttached` "/Game/Sounds/Monster_Storm.Monster_Storm" _box "None" (0.0 0.0 0.0) (struct) "KeepRelativeOffset" true 0.5 1.0 0.0 "/Game/Sounds/Attenuation/ATT_Monster.ATT_Monster" null))

(event `self.ReceiveTick`
  (params (DeltaSeconds :type "Float (single-precision)"))
  (if (`self.StartMoving`)
    (bind _returnvalue (`GameplayStatics.GetActorOfClass` "/Game/Blueprints/BP_MonsterSpawner.BP_MonsterSpawner_C"))
    (`self.K2_SetActorLocation` (`KismetMathLibrary.VInterpTo_Constant` (`self.K2_GetActorLocation`) (`self.K2_GetActorLocation` (`/Game/Blueprints/BP_MonsterSpawner.CurrentEndPoint` _returnvalue)) DeltaSeconds 500.0))))

(fn `UserConstructionScript`)